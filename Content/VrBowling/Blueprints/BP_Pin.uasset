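; VR bowling pin actor that plays a strike sound on ball contact and reports to the scoreboard.
; Any non-ball overlap on its Box calls DestroyPin, which toggles visibility and collision.
; A BP_ScoreBoard overlap then triggers PinOverlap through a DoOnce that is never reset.
; ResetPins calls DestroyPin and teleports the pin to the transform saved in the construction script.
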(event OnComponentBeginOverlap(Box)
  (params (OverlappedComponent :type Primitive%20Component%20Object%20Reference) (OtherActor :type Actor%20Object%20Reference) (OtherComp :type Primitive%20Component%20Object%20Reference) (OtherBodyIndex :type Integer) (bFromSweep :type Boolean) (SweepResult :type Hit%20Result%20Structure%20%28by%20ref%29))
  (if (Actor|ActorHasTag OtherActor "Ball")
    (CallFunction|StartPinSound)
    (else
      (CallFunction|DestroyPin (Variables|Rendering|GetbHidden))
      (bind _asbp_score_board (Utilities|Casting|CastToBP_ScoreBoard OtherActor))
      (Utilities|FlowControl|DoOnce false
        (:Completed
          (Default|PinOverlap _asbp_score_board))))))

(event Custom|ResetPins
  (CallFunction|DestroyPin (Variables|Rendering|GetbHidden))
  (Transformation|SetActorTransform (Variables|Default|GetStartTransform) false true))

(event Custom|StartPinSound
  (Audio|Components|Audio|Play (Variables|Default|GetAudio) 0.0))

(event Custom|DestroyPin
  (params (isHidden :type Boolean))
  (if isHidden
    (Rendering|SetActorHiddenInGame true)
    (Collision|SetActorEnableCollision false)
    (else
      (Rendering|SetActorHiddenInGame false)
      (Collision|SetActorEnableCollision true))))

(event EventBeginPlay
  (Audio|Components|Audio|SetSound (Variables|Default|GetAudio) "/Game/VrBowling/Assets/Sounds/BowlingStrike.BowlingStrike"))

(fn ConstructionScript
  (Variables|Default|SetStartTransform (Transformation|GetActorTransform)))