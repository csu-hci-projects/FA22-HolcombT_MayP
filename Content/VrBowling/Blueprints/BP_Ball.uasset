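; BP_Ball is the bowling ball in a VR bowling game, handling roll audio, hit notifications and respawning.
; Start and stop events control the roll sound, with a timed cutoff.
; Sphere overlaps trigger the pin sound on tagged BP_Pin actors or otherwise notify BP_ScoreBoard.
; ResetBall waits briefly, teleports to the construction-time transform, then toggles mesh mobility Static to Movable, apparently to clear motion.
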(event OnComponentBeginOverlap(Sphere)
  (params (OverlappedComponent :type Primitive%20Component%20Object%20Reference) (OtherActor :type Actor%20Object%20Reference) (OtherComp :type Primitive%20Component%20Object%20Reference) (OtherBodyIndex :type Integer) (bFromSweep :type Boolean) (SweepResult :type Hit%20Result%20Structure%20%28by%20ref%29))
  ;[1 1 1] If Ball hits a pin, call BP_Pin StartPinSound else if Ball hits the ScoreBoard, call BallOverlap
  (Utilities|IsValid OtherActor
    (:Is%20Valid
      (if (Actor|ActorHasTag OtherActor "Pin")
        (bind _asbp_pin (Utilities|Casting|CastToBP_Pin OtherActor))
        (Utilities|FlowControl|DoOnce false :!label _label
          (:Completed
            (Default|StartPinSound _asbp_pin)
            (goto _label Reset)))
        (else
          (bind _asbp_score_board (Utilities|Casting|CastToBP_ScoreBoard OtherActor))
          (Utilities|FlowControl|DoOnce false :!label _label_2
            (:Completed
              (Default|BallOverlap _asbp_score_board)
              (goto _label_2 Reset))))))))

(event Custom|ResetBall
  ;[1 1 1] ResetBall - Function is called elsewhere, resets ball to starting transform when triggered
  (Utilities|FlowControl|Delay 3.0)
  (Transformation|SetActorTransform (Variables|Default|GetStartTransform) false true)
  (Transformation|SetMobility (Variables|Default|GetStaticMesh) "Static")
  (Transformation|SetMobility (Variables|Default|GetStaticMesh) "Movable"))

(event Custom|StartRollSound
  (params (NewParam :type Rig%20Unit%20Get%20Delta%20Time%20Structure))
  ;[1 1 1] Set Ball sound and start/stop roll sound when triggered
  (Audio|Components|Audio|Play (Variables|Default|GetAudio) 0.0)
  (Utilities|FlowControl|Delay 15.0)
  (if (Audio|Components|Audio|IsPlaying (Variables|Default|GetAudio))
    (Audio|Components|Audio|Stop (Variables|Default|GetAudio))))

(event Custom|StopRollSound
  ;[1 1 1] Set Ball sound and start/stop roll sound when triggered
  (Audio|Components|Audio|Stop (Variables|Default|GetAudio)))

(event EventBeginPlay
  ;[1 1 1] Set Ball sound and start/stop roll sound when triggered
  (Audio|Components|Audio|SetSound (Variables|Default|GetAudio) "/Game/VrBowling/Assets/Sounds/BallRoll.BallRoll"))

(fn ConstructionScript
  ;[1 1 1] Set StartTransform
  (Variables|Default|SetStartTransform (Transformation|GetActorTransform)))