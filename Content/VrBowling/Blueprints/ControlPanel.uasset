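; VR bowling control panel with two physical buttons: one reloads the Bowling1 level, the other toggles the lane bumpers.
; Each trigger's overlap event checks for the VRPawn, animates its button down and back up, then opens the level or calls ToggleBumpers on the Bumpers actor.
; Both buttons share an IsPressed guard, which is set before the pawn check and never cleared here.
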(event OnComponentBeginOverlap(ResetTrigger)
  (params (OverlappedComponent :type Primitive%20Component%20Object%20Reference) (OtherActor :type Actor%20Object%20Reference) (OtherComp :type Primitive%20Component%20Object%20Reference) (OtherBodyIndex :type Integer) (bFromSweep :type Boolean) (SweepResult :type Hit%20Result%20Structure%20%28by%20ref%29))
  (bind _resetbutton (Variables|Default|GetResetButton))
  (bind _resetbutton_2 (Variables|Default|GetResetButton))
  (bind _returnvalue (Transformation|GetRelativeTransform _resetbutton_2))
  (bind _returnvalue_2 (Transformation|GetRelativeTransform _resetbutton))
  (if (not (Variables|Default|GetisPressed))
    (Variables|Default|SetisPressed true)
    (Utilities|Casting|CastToVRPawn OtherActor)
    (Components|MoveComponentTo _resetbutton (- (.location _returnvalue_2) "0,0,24.000000") (.rotation _returnvalue_2) false false 1.0 false)
    (Components|MoveComponentTo _resetbutton_2 (+ (.location _returnvalue) "0,0,24.000000") (.rotation _returnvalue) false false 1.0 false)
    (Game|OpenLevel(byObjectReference) "/Game/VrBowling/Maps/Bowling1.Bowling1")))

(event OnComponentBeginOverlap(BumperTrigger)
  (params (OverlappedComponent :type Primitive%20Component%20Object%20Reference) (OtherActor :type Actor%20Object%20Reference) (OtherComp :type Primitive%20Component%20Object%20Reference) (OtherBodyIndex :type Integer) (bFromSweep :type Boolean) (SweepResult :type Hit%20Result%20Structure%20%28by%20ref%29))
  (bind _bumperbutton (Variables|Default|GetBumperButton))
  (bind _bumperbutton_2 (Variables|Default|GetBumperButton))
  (bind _returnvalue (Transformation|GetRelativeTransform _bumperbutton_2))
  (bind _returnvalue_2 (Transformation|GetRelativeTransform _bumperbutton))
  (if (not (Variables|Default|GetisPressed))
    (Variables|Default|SetisPressed true)
    (Utilities|Casting|CastToVRPawn OtherActor)
    (Components|MoveComponentTo _bumperbutton (- (.location _returnvalue_2) "0,0,24.000000") (.rotation _returnvalue_2) false false 1.0 false)
    (Components|MoveComponentTo _bumperbutton_2 (+ (.location _returnvalue) "0,0,24.000000") (.rotation _returnvalue) false false 1.0 false)
    (bind _returnvalue_3 (Actor|GetActorOfClass "/Game/VrBowling/Blueprints/Bumpers.Bumpers_C"))
    (Default|ToggleBumpers _returnvalue_3)))

(fn ConstructionScript)