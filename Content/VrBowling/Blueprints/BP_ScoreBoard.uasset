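; BP_ScoreBoard is a VR bowling scoreboard that shows the score out of 300 and manages pin resets.
; Pin overlaps add a point each, and Tick rewrites the score text every frame.
; Every second ball overlap clears the throw count, waits five seconds, then resets pins matching the lane tag.
; Spare and Strike events flash a two-second message, but the strike check here is unconnected.
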(event Custom|Spare
  (bind _output_get (Variables|Default|SetFrame "Spare"))
  (Rendering|Components|TextRender|SetText (Variables|Default|GetAltText) _output_get)
  (Utilities|FlowControl|Delay 2.0)
  (bind _output_get_2 (Variables|Default|SetFrame ""))
  (Rendering|Components|TextRender|SetText (Variables|Default|GetAltText) _output_get_2))

(event Custom|Strike
  (bind _output_get (Variables|Default|SetFrame "Strike"))
  (Rendering|Components|TextRender|SetText (Variables|Default|GetAltText) _output_get)
  (Utilities|FlowControl|Delay 2.0)
  (bind _output_get_2 (Variables|Default|SetFrame ""))
  (Rendering|Components|TextRender|SetText (Variables|Default|GetAltText) _output_get_2))

(event Custom|BallOverlap
  (Variables|Default|SetBallsThrown (+ (Variables|Default|GetBallsThrown) 1))
  (if (>= (Variables|Default|GetBallsThrown) 2)
    (Variables|Default|SetBallsThrown 0)
    (Utilities|FlowControl|Delay 5.0)
    (bind _outactors (Actor|GetAllActorsOfClasswithTag "/Game/VrBowling/Blueprints/BP_Pin.BP_Pin_C" (Variables|Default|GetLane)))
    (for _array_element _outactors
      (Default|ResetPins _array_element))))

(event Custom|PinOverlap
  (Variables|Default|SetScore (+ (Variables|Default|GetScore) 1)))

(event EventTick
  (params (DeltaSeconds :type Float%20%28single-precision%29))
  (Rendering|Components|TextRender|SetText (Variables|Default|GetScoreText) (Utilities|Text|ToText(String) (Utilities|String|Append (Utilities|String|ToString(Text) (Utilities|Text|ToText(Integer) (Variables|Default|GetScore))) "/300"))))

(fn ConstructionScript)