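; Bumpers actor for VR bowling that can be switched on and off through its ToggleBumpers event.
; Each call flips the IsToggled flag and applies the new state to two static mesh components.
; When on, both meshes are visible and use PhysicsActor collision; when off, they are hidden in game with collision disabled.
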(event Custom|ToggleBumpers
  (bind _staticmesh1 (Variables|Default|GetStaticMesh1))
  (bind _staticmesh1_2 (Variables|Default|GetStaticMesh1))
  ;[1 1 1] ToggleBumpers - When triggered, toggles hidden in game and collision profile
  (if (Variables|Default|GetisToggled)
    (Variables|Default|SetisToggled false)
    (Development|SetHiddeninGame _staticmesh1 true false)
    (Collision|SetCollisionProfileName _staticmesh1 "NoCollision" true :!class /Script/Engine.PrimitiveComponent)
    (else
      (Variables|Default|SetisToggled true)
      (Development|SetHiddeninGame _staticmesh1_2 false false)
      (Collision|SetCollisionProfileName _staticmesh1_2 "PhysicsActor" true :!class /Script/Engine.PrimitiveComponent))))

(fn ConstructionScript)